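; Player controller for zombie mode that owns the player's HUD, pause menu and game over screen.
; On BeginPlay it creates the widgets and binds to FPS_Character_BP events for weapon switch, aiming, HUD updates and death.
; HUD updates refresh points and show buy or interact prompts from the hit actor, and aiming hides the crosshair, adding a scope for sniper rifles.
; Death shows game over stats from ZombieGameMode.
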(event `self.ReceiveBeginPlay`
  (bind _interactable_ui_ref (`self.Interactable UI ref`))
  (bind _buy_ui_ref (`self.Buy_UI_Ref`))
  (bind _interacthitactor (`FPS_Character.InteractHitActor` (`self.PawnRef`)))
  (bind _asfps_character_bp (cast `/Game/Dynamic/Player_Character/Behaviour/FPS_Character_BP` (`self.K2_GetPawn`)))
  (set `self.PawnRef` _asfps_character_bp)
  (`|ExecutionSequence`
    (:`then_0`
      (`self.Create Widgets`))
    (:`then_1`
      (add `FPS_Character.CharacterWeaponSwitch` (`self.PawnRef`) (delegate `Character weapon switch`)))
    (:`then_2`
      (add `FPS_Character.EventADSEnter` (`self.PawnRef`) (delegate `ADS enter`)))
    (:`then_3`
      (add `FPS_Character.EventADSExit` (`self.PawnRef`) (delegate `ADS exit`)))
    (:`then_4`
      (add `FPS_Character.UpdateWeaponHud` (`self.PawnRef`) (delegate `UpdateWeaponHud_Event_0`)))
    (:`then_5`
      (add `FPS_Character.EventPlayerDeath` (`self.PawnRef`) (delegate `EventPlayerDeath_Event`)))
    (:`then_6`
      (add `FPS_Character.UpdateMainHud` (`self.PawnRef`) (delegate `UpdateMainHud_Event_0`))
      (`/Game/Dynamic/UI/PlayerMainUI/Health-Armor_Widget.Update Points` (`/Game/Dynamic/UI/PlayerMainUI/ZombieModeMain_Widget.Health-Armor_UI` (`self.MainHUD ref`)) (`FPS_Character.GetPoints` (`self.PawnRef`)) :!label _label)
      (`/Engine/EditorBlueprintResources/StandardMacros.IsValid` _interacthitactor
        (:`Is Valid`
          (bind _asinteractables (cast `Interactables` _interacthitactor)
            (:`then`
              (bind _asbuyable_object (cast `BuyableObject` _asinteractables)
                (:`then`
                  (if (`Widget.IsInViewport` _buy_ui_ref)
                    (`Widget.RemoveFromParent` _buy_ui_ref))
                  (`UserWidget.AddToViewport` _buy_ui_ref 0)
                  (`/Game/Dynamic/UI/PlayerMainUI/Buy_Widget.UpdateData1` _buy_ui_ref (`BuyableObject.Cost` _asbuyable_object) (`Interactables.InteractableText` _asbuyable_object)))
                (:`CastFailed`
                  (if (`Widget.IsInViewport` _interactable_ui_ref)
                    (`Widget.RemoveFromParent` _interactable_ui_ref))
                  (`UserWidget.AddToViewport` _interactable_ui_ref 0)
                  (`/Game/Dynamic/UI/PlayerMainUI/Interactable_Widget.UpdateData1` _interactable_ui_ref (`Interactables.InteractableText` _asinteractables)))))
            (:`CastFailed`
              (`|ExecutionSequence` :!label _label_2
                (:`then_0`
                  (if (`Widget.IsInViewport` (`self.Buy_UI_Ref`))
                    (`Widget.RemoveFromParent` (`self.Buy_UI_Ref`))))
                (:`then_1`
                  (if (`Widget.IsInViewport` (`self.Interactable UI ref`))
                    (`Widget.RemoveFromParent` (`self.Interactable UI ref`))))))))
        (:`Is Not Valid`
          (goto _label_2))))))

(event `Character weapon switch`
  (`/Game/Dynamic/UI/PlayerMainUI/DynamicCrosshair_Widget.UpdateCrosshair` (`/Game/Dynamic/UI/PlayerMainUI/ZombieModeMain_Widget.DynamicCrosshair` (`self.MainHUD ref`))))

(event `InputAction|Pause Menu`
  (params (Key :type "Key Structure"))
  (:`Pressed`
    (`WidgetBlueprintLibrary.SetInputMode_UIOnlyEx` self null)
    (set `self.bShowMouseCursor` true)
    (`UserWidget.AddToViewport` (`self.PauseMenuRef`) 0)
    (`GameplayStatics.SetGamePaused` true)))

(event `ADS enter`
  (`self.ADS HUD Enter`))

(event `ADS exit`
  (`self.ADS HUD Exit`))

(event `UpdateWeaponHud_Event_0`
  (bind _ui_weaponinfo (`/Game/Dynamic/UI/PlayerMainUI/ZombieModeMain_Widget.UI_WeaponInfo` (`self.MainHUD ref`)))
  (bind _currentweapon (`FPS_Character.CurrentWeapon` (`self.PawnRef`)))
  (`/Engine/EditorBlueprintResources/StandardMacros.IsValid` _currentweapon
    (:`Is Valid`
      (`Widget.SetVisibility` _ui_weaponinfo "Visible")
      (`/Game/Dynamic/UI/PlayerMainUI/WeaponInfo_Widget.GetCurrentWeapon` _ui_weaponinfo _currentweapon)
      (`/Game/Dynamic/UI/PlayerMainUI/WeaponInfo_Widget.GetReloading` _ui_weaponinfo (`FPS_Character.bIsReloading` (`self.PawnRef`))))
    (:`Is Not Valid`
      (`Widget.SetVisibility` _ui_weaponinfo "Collapsed"))))

(event `UpdateMainHud_Event_0`
  (goto _label))

(event `EventPlayerDeath_Event`
  (`Widget.SetVisibility` (`self.MainHUD ref`) "Collapsed")
  (`self.CreateGameOverWidget`))

(fn `ADS HUD Enter`
  (bind _sniperscope_ref (`self.SniperScope ref`))
  (`Widget.SetVisibility` (`/Game/Dynamic/UI/PlayerMainUI/ZombieModeMain_Widget.DynamicCrosshair` (`self.MainHUD ref`)) "Collapsed")
  (if (`|EnumEquality` (`WeaponBase.WeaponType` (`FPS_Character.CurrentWeapon` (`self.PawnRef`))) "SniperRifle")
    (if (not (`Widget.IsInViewport` _sniperscope_ref))
      (`UserWidget.AddToViewport` _sniperscope_ref 0))))

(fn `ADS HUD Exit`
  (bind _sniperscope_ref (`self.SniperScope ref`))
  (`Widget.SetVisibility` (`/Game/Dynamic/UI/PlayerMainUI/ZombieModeMain_Widget.DynamicCrosshair` (`self.MainHUD ref`)) "Visible")
  (if (`Widget.IsInViewport` _sniperscope_ref)
    (`Widget.RemoveFromParent` _sniperscope_ref)))

(fn `Create Widgets`
  (`|ExecutionSequence`
    (:`then_0`
      (bind _returnvalue (`|CreateWidget` "/Game/Dynamic/UI/PlayerMainUI/ZombieModeMain_Widget.ZombieModeMain_Widget_C"))
      (bind _output_get (set `self.MainHUD ref` _returnvalue))
      (`UserWidget.AddToViewport` _output_get 0))
    (:`then_1`
      (bind _returnvalue_2 (`|CreateWidget` "/Game/Dynamic/UI/PlayerMainUI/Buy_Widget.Buy_Widget_C"))
      (set `self.Buy_UI_Ref` _returnvalue_2))
    (:`then_2`
      (bind _returnvalue_3 (`|CreateWidget` "/Game/Dynamic/UI/PlayerMainUI/SniperScope_Widget.SniperScope_Widget_C"))
      (set `self.SniperScope ref` _returnvalue_3))
    (:`then_3`
      (bind _returnvalue_4 (`|CreateWidget` "/Game/Dynamic/UI/PlayerMainUI/Interactable_Widget.Interactable_Widget_C"))
      (set `self.Interactable UI ref` _returnvalue_4))
    (:`then_4`
      (bind _returnvalue_5 (`|CreateWidget` "/Game/Dynamic/UI/MenuScreensUI/PauseMenu_UI.PauseMenu_UI_C"))
      (set `self.PauseMenuRef` _returnvalue_5))))

(fn `CreateGameOverWidget`
  (bind _aszombie_game_mode (cast `ZombieGameMode` (`GameplayStatics.GetGameMode`)))
  (bind _returnvalue (`|CreateWidget` "/Game/Dynamic/UI/PlayerMainUI/ZombieMode_GameOver_Widget.ZombieMode_GameOver_Widget_C" null (`ZombieGameMode.GetZombiesKilled` _aszombie_game_mode) (`ZombieGameMode.GetTotalScore` _aszombie_game_mode) (`ZombieGameMode.GetCurrentRound` _aszombie_game_mode)))
  (`UserWidget.AddToViewport` _returnvalue 0)
  (`WidgetBlueprintLibrary.SetInputMode_UIOnlyEx` self _returnvalue)
  (set `self.bShowMouseCursor` true))

(fn `UserConstructionScript`)